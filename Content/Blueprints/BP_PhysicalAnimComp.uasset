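; Component that adds physical animation to its owning BP_TopDownCharacter, set up for hit reactions.
; On BeginPlay it creates a PhysicalAnimationComponent on the character and binds it to the skeletal mesh.
; TogglePhysicalAnimation, despite its name, has no off branch: it enables physics simulation from the pelvis down the bone chain, applies HitReactionProfile and sets strength and physics blend weight.
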(event `self.ReceiveBeginPlay`
  (bind _asbp_top_down_character (cast `/Game/TopDown/Blueprints/BP_TopDownCharacter` (`self.GetOwner`)))
  (bind _mesh (`Character.Mesh` _asbp_top_down_character))
  (set `self.Mesh` _mesh)
  (bind _returnvalue (`|AddComponentByClass` _asbp_top_down_character "/Script/Engine.PhysicalAnimationComponent"))
  (bind _output_get (set `self.PhysicalAnimationComponent` _returnvalue))
  (`PhysicalAnimationComponent.SetSkeletalMeshComponent` _output_get _mesh))

(event `TogglePhysicalAnimation`
  (bind _physicalanimationcomponent (`self.PhysicalAnimationComponent`))
  (`SkeletalMeshComponent.SetAllBodiesBelowSimulatePhysics` (`self.Mesh`) "pelvis" true true)
  (`PhysicalAnimationComponent.ApplyPhysicalAnimationProfileBelow` _physicalanimationcomponent "pelvis" "HitReactionProfile" true false)
  (`PhysicalAnimationComponent.SetStrengthMultiplyer` _physicalanimationcomponent 1.0)
  (`SkeletalMeshComponent.SetAllBodiesBelowPhysicsBlendWeight` (`self.Mesh`) "pelvis" 0.0 false true))