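; BP_Panelak1 is a building actor assembled from static mesh components, including a ground-floor door frame, top floor and rooftop cabin.
; Its construction script walks all descendants of the root and writes the Color variable into the "Color" material parameter of static mesh components, tinting the building as a whole.
; The cast exits at the first non-static-mesh child, and the event graph holds no active logic.
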(fn `UserConstructionScript`
  (for _array_element (`SceneComponent.GetChildrenComponents` (`self.DefaultSceneRoot`) true)
    (bind _asstatic_mesh_component (cast `StaticMeshComponent` _array_element))
    (`MeshComponent.SetVectorParameterValueOnMaterials` _asstatic_mesh_component "Color" (`KismetMathLibrary.Conv_LinearColorToVector` (`self.Color`)))))