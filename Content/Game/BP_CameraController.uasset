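; Player controller for a map camera that pans with directional inputs or screen-edge mouse scrolling and zooms with the mouse wheel.
; BeginPlay measures the Map actor's bounds, shows the cursor and locks it to the viewport.
; Each tick, MoveCamera smooths zoom, which drives pan speed, pitch and BP_CameraPawn's spring arm length.
; The pawn stays at fixed height, clamped to map size; movement is not scaled by delta time.
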(event `self.ReceiveBeginPlay`
  (set `self.CameraPawn` (`GameplayStatics.GetPlayerPawn` 0))
  (bind _returnvalue (`GameplayStatics.GetActorOfClass` "/Game/Game/Map.Map_C"))
  (bind _output_get (set `self.Map` _returnvalue))
  (bind (_origin _boxextent) (`self.GetActorBounds` _output_get false false))
  (set `self.GridXSize` (* (.x _boxextent) 2.0))
  (set `self.GridYSize` (* (.y _boxextent) 2.0))
  (`WidgetBlueprintLibrary.SetInputMode_GameAndUIEx` self null "LockAlways" false)
  (set `self.bShowMouseCursor` true))

(event `self.ReceiveTick`
  (params (DeltaSeconds :type "Float (single-precision)"))
  (`self.MoveCamera`))

(event `InputAction|Left`
  (params (Key :type "Key Structure"))
  (bind _cameramovement (`self.CameraMovement`))
  ;[1 1 1] MoveCameraLeft
  (:`Pressed`
    (set `self.CameraMovement` (- _cameramovement (0.0 1.0 0.0))))
  (:`Released`
    (set `self.CameraMovement` (+ _cameramovement (0.0 1.0 0.0)))))

(event `InputAction|Up`
  (params (Key :type "Key Structure"))
  (bind _cameramovement (`self.CameraMovement`))
  ;[1 1 1] MoveCameraUp
  (:`Pressed`
    (set `self.CameraMovement` (+ _cameramovement (1.0 0.0 0.0))))
  (:`Released`
    (set `self.CameraMovement` (- _cameramovement (1.0 0.0 0.0)))))

(event `InputAction|Right`
  (params (Key :type "Key Structure"))
  (bind _cameramovement (`self.CameraMovement`))
  ;[1 1 1] MoveCameraRight
  (:`Pressed`
    (set `self.CameraMovement` (+ _cameramovement (0.0 1.0 0.0))))
  (:`Released`
    (set `self.CameraMovement` (- _cameramovement (0.0 1.0 0.0)))))

(event `InputAction|Down`
  (params (Key :type "Key Structure"))
  (bind _cameramovement (`self.CameraMovement`))
  ;[1 1 1] MoveCameraDown
  (:`Pressed`
    (set `self.CameraMovement` (- _cameramovement (1.0 0.0 0.0))))
  (:`Released`
    (set `self.CameraMovement` (+ _cameramovement (1.0 0.0 0.0)))))

(event `Key|MouseScrollUp`
  (params (Key :type "Key Structure"))
  ;[1 1 1] CameraZoom
  (:`Pressed`
    (set `self.CameraZoom` (`KismetMathLibrary.FClamp` (- (`self.CameraZoom`) 0.1)))))

(event `Key|MouseScrollDown`
  (params (Key :type "Key Structure"))
  ;[1 1 1] CameraZoom
  (:`Pressed`
    (set `self.CameraZoom` (`KismetMathLibrary.FClamp` (+ (`self.CameraZoom`) 0.1)))))

(fn `MoveCamera`
  (bind _returnvalue_x (`KismetMathLibrary.BreakVector2D` (`WidgetLayoutLibrary.GetViewportSize`)))
  (bind (_returnvalue_x_2 _returnvalue_y) (`KismetMathLibrary.BreakVector2D` (`WidgetLayoutLibrary.GetViewportSize`)))
  (bind _returnvalue_x_3 (`KismetMathLibrary.BreakVector2D` (`WidgetLayoutLibrary.GetViewportSize`)))
  (bind (_returnvalue_x_4 _returnvalue_y_2) (`KismetMathLibrary.BreakVector2D` (`WidgetLayoutLibrary.GetViewportSize`)))
  (bind _camerapawn (`self.CameraPawn`))
  (bind (_returnvalue_x_5 _returnvalue_y_3) (`KismetMathLibrary.BreakVector` (+ (`self.K2_GetActorLocation` _camerapawn) (* (`KismetMathLibrary.Normal` (- (`KismetMathLibrary.Normal` (`self.CameraMovement`)) (`KismetMathLibrary.MakeVector` 0.0 (- 1.0 (`KismetMathLibrary.FClamp` (`KismetMathLibrary.NormalizeToRange` (`self.MouseX`) 0.0 (* _returnvalue_x 0.005))))) (`KismetMathLibrary.MakeVector` 0.0 (* (`KismetMathLibrary.FClamp` (`KismetMathLibrary.NormalizeToRange` (`self.MouseX`) (* _returnvalue_x_3 1.0) _returnvalue_x_3)) -1.0)) (* (`KismetMathLibrary.MakeVector` (- 1.0 (`KismetMathLibrary.FClamp` (`KismetMathLibrary.NormalizeToRange` (`self.MouseY`) 0.0 (* _returnvalue_y_2 0.005))))) -1.0) (* (`KismetMathLibrary.MakeVector` (* (`KismetMathLibrary.FClamp` (`KismetMathLibrary.NormalizeToRange` (`self.MouseY`) (* _returnvalue_y 0.999999) _returnvalue_y)) -1.0)) -1.0))) (`KismetMathLibrary.Lerp` (`self.MinCameraSpeed`) (`self.MaxCameraSpeed`) (`self.CurrentCameraZoom`))))))
  (set `self.CurrentCameraZoom` (`KismetMathLibrary.FInterpTo` (`self.CurrentCameraZoom`) (`self.CameraZoom`) (`GameplayStatics.GetWorldDeltaSeconds`) 5.0))
  (bind _returnvalue (`WidgetLayoutLibrary.GetMousePositionOnViewport`))
  (set `self.MouseX` (`KismetMathLibrary.BreakVector2D` _returnvalue))
  (set `self.MouseY` (`.Y` (`KismetMathLibrary.BreakVector2D` _returnvalue)))
  (`self.K2_SetActorLocationAndRotation` _camerapawn (`KismetMathLibrary.MakeVector` (`KismetMathLibrary.FClamp` _returnvalue_x_5 0.0 (`self.GridXSize`)) (`KismetMathLibrary.FClamp` _returnvalue_y_3 0.0 (`self.GridYSize`)) 250.0) (`KismetMathLibrary.MakeRotator` 0.0 (`KismetMathLibrary.Lerp` 30.0 0.0 (`self.CurrentCameraZoom`))) false false)
  (bind _asbp_camera_pawn (cast `/Game/Game/BP_CameraPawn` (`self.CameraPawn`)))
  (set `SpringArmComponent.TargetArmLength` (`KismetMathLibrary.Lerp` (`self.MinZoomDistance`) (`self.MaxZoomDistance`) (`self.CurrentCameraZoom`)) (`/Game/Game/BP_CameraPawn.SpringArm` _asbp_camera_pawn)))

(fn `UserConstructionScript`)