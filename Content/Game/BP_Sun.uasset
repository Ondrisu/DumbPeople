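; BP_Sun is a sun actor that drives the day-night cycle by rotating its directional light.
; Each tick it adds local pitch scaled by delta time and CurrentSpeed, then tests the light's world pitch against a fixed range to set IsNight.
; CurrentSpeed eases toward NightSpeed or DaySpeed with FInterpTo, so night and day can pass at different rates without an abrupt change.
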(event `self.ReceiveTick`
  (params (DeltaSeconds :type "Float (single-precision)"))
  (bind _directionallight (`self.DirectionalLight`))
  (bind (_returnvalue_roll _returnvalue_pitch) (`KismetMathLibrary.BreakRotator` (`SceneComponent.K2_GetComponentRotation` _directionallight)))
  (`SceneComponent.K2_AddLocalRotation` _directionallight (`KismetMathLibrary.MakeRotator` 0.0 (* DeltaSeconds (`self.CurrentSpeed`))) false false)
  (if (and (>= _returnvalue_pitch -10.0) (<= _returnvalue_pitch 200.0))
    (set `self.IsNight` true)
    (set `self.CurrentSpeed` (`KismetMathLibrary.FInterpTo` (`self.CurrentSpeed`) (`self.NightSpeed`) (`GameplayStatics.GetWorldDeltaSeconds`) 1.0))
    (else
      (set `self.IsNight` false)
      (set `self.CurrentSpeed` (`KismetMathLibrary.FInterpTo` (`self.CurrentSpeed`) (`self.DaySpeed`) (`GameplayStatics.GetWorldDeltaSeconds`) 1.0)))))

(fn `UserConstructionScript`)