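; Base human AI character Blueprint that provides physically animated bodies and a set of movement actions.
; On BeginPlay it applies a physical animation profile and simulates physics on bodies below a chosen bone.
; Events jump by launch arc, slide via timeline lerp, teleport, or push away from an attacker by impulse.
; SetMovementSpeed maps a speed state to walk speed; GetPatrolRoute is empty and the AIMoveTo follow loop is unconnected.
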(event `self.ReceiveBeginPlay`
  (`self.WalkingState`))

(event `WalkingState`
  (bind _bone (`self.Bone`))
  (`PhysicalAnimationComponent.SetSkeletalMeshComponent` (`self.PhysicalAnimation`) (`self.Mesh`))
  (`PhysicalAnimationComponent.ApplyPhysicalAnimationProfileBelow` (`self.PhysicalAnimation`) _bone "Normal" false true)
  (`SkeletalMeshComponent.SetAllBodiesBelowSimulatePhysics` (`self.Mesh`) _bone true false))

(event `/Game/Human/AI/BPI_Human.JumpToLocation`
  (params (Location :type "Vector Structure"))
  (bind _outlaunchvelocity (`GameplayStatics.SuggestProjectileVelocity_CustomArc` (`self.K2_GetActorLocation`) (`KismetMathLibrary.MakeVector` (.x Location) (.y Location) (+ (.z Location) 1000.0))))
  (`self.LaunchCharacter` _outlaunchvelocity true true))

(event `/Game/Human/AI/BPI_Human.MoveToLocation`
  (params (Location :type "Vector Structure"))
  (bind (_direction _movelength) (`Timeline|MoveToLocationTimeLine` :!via `PlayFromStart`)
    (:`Update`
      (`self.K2_SetActorLocation` (`KismetMathLibrary.VLerp` Location (`self.K2_GetActorLocation`) _movelength) true))))

(event `/Game/Human/AI/BPI_Human.TeleportToLocation`
  (params (Location :type "Vector Structure"))
  (`self.K2_TeleportTo` self (`KismetMathLibrary.MakeVector` Location_X Location_Y (+ Location_Z 200.0)) (`self.K2_GetActorRotation`)))

(event `/Game/Human/AI/BPI_Human.PushAway`
  (params (LocationOfAttacker :type "Vector Structure"))
  (bind (_returnvalue_x _returnvalue_y _returnvalue_z) (`KismetMathLibrary.BreakVector` (* (`KismetMathLibrary.Normal` (- (`self.K2_GetActorLocation`) LocationOfAttacker)) 2000.0)))
  (bind _returnvalue_x_2 (`KismetMathLibrary.BreakVector2D` (`KismetMathLibrary.ClampAxes2D` (`KismetMathLibrary.Conv_DoubleToVector2D` _returnvalue_z) 0.0 _returnvalue_z)))
  (`CharacterMovementComponent.AddImpulse` (`self.CharacterMovement`) (`KismetMathLibrary.MakeVector` _returnvalue_x _returnvalue_y _returnvalue_x_2) true))

(fn `GetPatrolRoute`)

(fn `SetMovementSpeed`
  (params (Speed :type "/Game/Human/AI/Enums/E_MovementSpeed Enum" :default "NewEnumerator0"))
  (returns (SpeedValue :type "Float (double-precision)"))
  (set `CharacterMovementComponent.MaxWalkSpeed` (select `/Game/Human/AI/Enums/E_MovementSpeed` Speed :`NewEnumerator1` 250.0 :`NewEnumerator3` 350.0 :`NewEnumerator2` 500.0 :!type "Float (single-precision)") (`self.CharacterMovement`))
  (return 0.0))

(fn `UserConstructionScript`)