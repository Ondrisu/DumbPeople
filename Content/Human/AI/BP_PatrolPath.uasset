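; Patrol path for human AI that supplies world-space waypoints from the points of its Path spline.
; GetSplinePointAsWorldPosition returns the point at the current PatrolIndex, and InceremntPatrolRoute steps that index by PatrolDirection.
; The direction flips at the last and first points for a back-and-forth route, with the progress stored on the path itself rather than passed in by callers.
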(event `InceremntPatrolRoute`
  (bind _output_get (set `self.PatrolIndex` (+ (`self.PatrolIndex`) (`self.PatrolDirection`))))
  (if (== _output_get (- (`SplineComponent.GetNumberOfSplinePoints` (`self.Path`)) 1))
    (set `self.PatrolDirection` -1)
    (elif (== (`self.PatrolIndex`) 0)
      (set `self.PatrolDirection` 1))))

(fn `GetSplinePointAsWorldPosition`
  (returns (Location :type "Vector Structure"))
  (return (`SplineComponent.GetLocationAtSplinePoint` (`self.Path`) (`self.PatrolIndex`) "World")))

(fn `UserConstructionScript`)