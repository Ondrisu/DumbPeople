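; BP_BaseRock is a rock prop that can be knocked away from an attacker.
; Its construction script randomizes a dark material color, yaw and uniform scale for visual variety.
; The PushAway event applies a fixed-strength impulse to the Rock component, directed away from the attacker's location.
; GetPatrolRoute and SetMovementSpeed are empty stubs with no patrol or movement logic.
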(event `self.PushAway`
  (params (LocationOfAttacker :type "Vector Structure"))
  (`PrimitiveComponent.AddImpulse` (`self.Rock`) (* (`KismetMathLibrary.Normal` (- (`self.K2_GetActorLocation`) LocationOfAttacker)) 2000.0) "None" false))

(fn `GetPatrolRoute`
  (returns (PatrolRoute :type "/Game/Human/AI/BP_PatrolPath Object Reference"))
  (return null))

(fn `SetMovementSpeed`
  (params (Speed :type "/Game/Human/AI/Enums/E_MovementSpeed Enum" :default "NewEnumerator0"))
  (returns (SpeedValue :type "Float (double-precision)"))
  (return 0.0))

(fn `UserConstructionScript`
  (bind _returnvalue (`KismetMathLibrary.RandomFloatInRange` 0.03 0.3))
  (bind _rock (`self.Rock`))
  (bind _output_get (set `self.Color` (make `LinearColor` _returnvalue _returnvalue _returnvalue)))
  (`MeshComponent.SetVectorParameterValueOnMaterials` _rock "Color" (`KismetMathLibrary.Conv_LinearColorToVector` _output_get))
  (`SceneComponent.K2_SetWorldRotation` _rock (`KismetMathLibrary.MakeRotator` 0.0 0.0 (`KismetMathLibrary.RandomFloatInRange` 0.0 360.0)) false true)
  (`SceneComponent.SetWorldScale3D` _rock (`KismetMathLibrary.Conv_DoubleToVector` (`KismetMathLibrary.RandomFloatInRange` 0.8 1.5))))