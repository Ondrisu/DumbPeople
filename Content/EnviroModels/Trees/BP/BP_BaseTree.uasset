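; Base tree actor whose skeletal mesh sways physically and can be knocked away from an attacker.
; BeginPlay simulates bodies below a named bone, driven by the "Normal" physical animation profile.
; PushAway applies an impulse to those bodies, directed away from the attacker's location.
; The construction script randomizes green shade, yaw and uniform scale; GetPatrolRoute and SetMovementSpeed are empty stubs.
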(event `self.ReceiveBeginPlay`
  (`PhysicalAnimationComponent.SetSkeletalMeshComponent` (`self.PhysicalAnimation`) (`self.Tree`))
  (`PhysicalAnimationComponent.ApplyPhysicalAnimationProfileBelow` (`self.PhysicalAnimation`) (`self.Body Name`) "Normal" false true)
  (`SkeletalMeshComponent.SetAllBodiesBelowSimulatePhysics` (`self.Tree`) (`self.Body Name`) true false))

(event `/Game/Human/AI/BPI_Human.PushAway`
  (params (LocationOfAttacker :type "Vector Structure"))
  (`SkeletalMeshComponent.AddImpulseToAllBodiesBelow` (`self.Tree`) (* (`KismetMathLibrary.Normal` (- (`self.K2_GetActorLocation`) LocationOfAttacker)) 2000.0) (`self.Body Name`) true true))

(fn `GetPatrolRoute`
  (returns (PatrolRoute :type "/Game/Human/AI/BP_PatrolPath Object Reference"))
  (return null))

(fn `SetMovementSpeed`
  (params (Speed :type "/Game/Human/AI/Enums/E_MovementSpeed Enum" :default "NewEnumerator0"))
  (returns (SpeedValue :type "Float (double-precision)"))
  (return 0.0))

(fn `UserConstructionScript`
  (bind _tree (`self.Tree`))
  (bind _output_get (set `self.Color` (make `LinearColor` 0.0 (`KismetMathLibrary.RandomFloatInRange` 0.03 0.3) 0.0 1.0)))
  (`MeshComponent.SetVectorParameterValueOnMaterials` (`self.Tree`) "Color" (`KismetMathLibrary.Conv_LinearColorToVector` _output_get))
  (`SceneComponent.K2_SetWorldRotation` _tree (`KismetMathLibrary.MakeRotator` 0.0 0.0 (`KismetMathLibrary.RandomFloatInRange` 0.0 360.0)) false true)
  (`SceneComponent.SetWorldScale3D` _tree (`KismetMathLibrary.Conv_DoubleToVector` (`KismetMathLibrary.RandomFloatInRange` 0.8 1.5))))